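; BPC_Attacks is an attack component that gives its owner a hitscan bullet and a targeted magic arrow projectile.
; FireBullet line-traces for Pawns with debug drawing, while MagicSpell spawns the arrow, ignoring its owner, and binds its impact event.
; Both send hits a damage message and report a damage event, likely for AI perception.
; Only projectile impact broadcasts OnAttackEnded, reusing the DamageInfo passed to MagicSpell.
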(event `FireBullet`
  (params (TraceStart :type "Vector Structure") (TraceEnd :type "Vector Structure") (DamageInfo :type "/Game/DamageSystem/Structure/S_DamageInfo Structure"))
  (bind (_outhit _returnvalue) (`KismetSystemLibrary.LineTraceSingleForObjects` :`Start` TraceStart :`End` TraceEnd :`ObjectTypes` (`|MakeArray` "ObjectTypeQuery3" :!type "EObjectTypeQuery Enum") :`DrawDebugType` "ForDuration"))
  (if _returnvalue
    (bind (_bblockinghit _binitialoverlap _time _distance _location _impactpoint _normal _impactnormal _physmat _hitactor) (`GameplayStatics.BreakHitResult` _outhit))
    (message `/Game/DamageSystem/Interface/BPI_Damagalbe.TakeDamage` _hitactor DamageInfo (`self.GetOwner`))
    (`AISense_Damage.ReportDamageEvent` _hitactor (`self.GetOwner`) (`.Amount_2_B8D4B704400F439FF668E78A15F55AD3` (break `/Game/DamageSystem/Structure/S_DamageInfo` DamageInfo)) (`Actor.K2_GetActorLocation` (`self.GetOwner`)))))

(event `MagicSpell`
  (params (SpawnTransform :type "Transform Structure") (Target :type "Actor Object Reference") (DamageInfo :type "/Game/DamageSystem/Structure/S_DamageInfo Structure"))
  (bind _returnvalue (`|SpawnActorFromClass` "/Game/Projectile/BP_Projectile_MagicArrow.BP_Projectile_MagicArrow_C" SpawnTransform "Undefined" "MultiplyWithRoot" (`self.GetOwner`) 1000.0 0.0 Target false null))
  (add `/Game/Projectile/BP_Projectile_Base.OnProjectileImpact` _returnvalue (delegate `OnProjectileHit`))
  (`PrimitiveComponent.IgnoreActorWhenMoving` (`/Game/Projectile/BP_Projectile_Base.BoxCollision` _returnvalue) (`self.GetOwner`) true))

(event `OnProjectileHit`
  (params (`Other Actor` :type "Actor Object Reference") (Hit :type "HitResult Structure"))
  (message `/Game/DamageSystem/Interface/BPI_Damagalbe.TakeDamage` `Other Actor` (stale `MagicSpell` DamageInfo) (`self.GetOwner`))
  (`AISense_Damage.ReportDamageEvent` `Other Actor` (`self.GetOwner`) (`.Amount_2_B8D4B704400F439FF668E78A15F55AD3` (break `/Game/DamageSystem/Structure/S_DamageInfo` (stale `MagicSpell` DamageInfo))) (`Actor.K2_GetActorLocation` (`self.GetOwner`)))
  (`self.OnAttackEnded`))