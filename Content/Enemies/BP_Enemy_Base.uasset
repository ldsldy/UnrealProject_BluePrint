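; Base enemy character with sword-and-shield combat actions and movement helpers.
; Attack, WieldSword and SheathSword play montages, with dispatchers reporting when the attack ends or the draw and sheath complete.
; Montage notifies time the spawning and attaching of the sword to the hand socket, and its destruction on sheathing, while updating the wielding flag.
; Functions supply attack and defense radii and the patrol route, and map movement states to walk speeds.
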(event `self.ReceiveBeginPlay`)

(event `Attack`
  (`|PlayMontage` (`self.Mesh`) "/Game/Animations/Sword/AM_Sword_And_Shield_Slash_Anim1_Montage.AM_Sword_And_Shield_Slash_Anim1_Montage"
    (:`OnCompleted`
      _)
    (:`OnInterrupted`
      _))
  (`self.OnAttackEnd`))

(event `WieldSword`
  ; 검을 뽑으면서 검을 생성
  (bind _notifyname (`|PlayMontage` (`self.Mesh`) "/Game/Animations/Sword/AM_Draw_Sword.AM_Draw_Sword")
    (:`OnCompleted`
      (`self.OnWieldSword`))
    (:`OnNotifyBegin`
      (switch `name` _notifyname
        (:`HoldSword`
          (bind _returnvalue (`|SpawnActorFromClass` "/Game/Weapon/BP_EnemySword.BP_EnemySword_C" (`self.GetTransform`) "AlwaysSpawn" "MultiplyWithRoot" null null))
          (bind _output_get (set `self.Sword Actor` _returnvalue))
          (`self.K2_AttachToComponent` _output_get (`self.Mesh`) "hand_r_sword_socket" "SnapToTarget" "SnapToTarget" "SnapToTarget" true)
          (set `self.IsWieldingSword` true))))))

(event `SheathSword`
  ; 검을 집어 넣으면서 검을 삭제
  (bind _notifyname (`|PlayMontage` (`self.Mesh`) "/Game/Animations/Sword/AM_Sheath_Sword.AM_Sheath_Sword")
    (:`OnCompleted`
      (`self.OnSheathSword`))
    (:`OnNotifyBegin`
      (switch `name` _notifyname
        (:`DropSword`
          (`self.K2_DestroyActor` (`self.Sword Actor`))
          (set `self.IsWieldingSword` false))))))

(fn `GetIdealRange`
  (returns (AttackRadius :type "Float (double-precision)") (DefenseRadius :type "Float (double-precision)"))
  (return 150.0 350.0))

(fn `GetPatrolRoute`
  (returns (PatrolRoute :type "/Game/Enemies/BP_PatrolRoute Object Reference"))
  (return (`self.PatrolRoute`)))

(fn `SetMovementSpeed`
  (params (State :type "/Game/Enums/E_MovementState Enum" :default "NewEnumerator0"))
  (returns (Speed :type "Float (double-precision)"))
  (bind _output_get (set `CharacterMovementComponent.MaxWalkSpeed` (select `/Game/Enums/E_MovementState` State :`NewEnumerator1` 100.0 :`NewEnumerator2` 300.0 :`NewEnumerator3` 500.0) (`self.CharacterMovement`)))
  (return _output_get))

(fn `UserConstructionScript`)