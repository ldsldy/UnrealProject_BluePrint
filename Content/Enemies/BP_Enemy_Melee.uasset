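; Melee enemy Blueprint child that fights with a sword, overriding attack, equip and unequip events.
; The attack montage's notify fires a forward sphere trace against pawns and sends damage to the hit actor.
; The damage system is uninterruptible during the swing (super armor), restored on completion or interruption.
; Draw and sheath montage notifies spawn and attach the sword or destroy it, with completion calling weapon state dispatchers.
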(event `self.ReceiveBeginPlay`
  (`parent.ReceiveBeginPlay`))

(event `/Game/Enemies/Interfaces/BPI_EnemyAI.DefaultAttack`
  (bind _returnvalue (`self.K2_GetActorLocation`))
  (bind _notifyname (`|PlayMontage` (`self.Mesh`) "/Game/Animations/SwordAction/AM_Sword_And_Shield_Slash_Anim1_Montage.AM_Sword_And_Shield_Slash_Anim1_Montage")
    (:`then`
      ; 공격하는 동안은 슈퍼아머
      (set `/Game/DamageSystem/Blueprints/BPC_DamageSystem.IsInterruptible` false (`self.BPC_DamageSystem`)))
    (:`OnCompleted`
      (`self.OnAttackEnd` :!label _label)
      (set `/Game/DamageSystem/Blueprints/BPC_DamageSystem.IsInterruptible` true (`self.BPC_DamageSystem`)))
    (:`OnInterrupted`
      (goto _label))
    (:`OnNotifyBegin`
      (switch `name` _notifyname
        (:`Slash`
          (bind (_outhit _returnvalue_2) (`KismetSystemLibrary.SphereTraceSingleForObjects` :`Start` _returnvalue :`End` (+ _returnvalue (* (`self.GetActorForwardVector`) 200.0)) :`ObjectTypes` (`|MakeArray` "ObjectTypeQuery3" :!type "EObjectTypeQuery Enum") :`DrawDebugType` "ForDuration"))
          (if _returnvalue_2
            (message `/Game/DamageSystem/Interface/BPI_Damagalbe.TakeDamage` (`.HitActor` (`GameplayStatics.BreakHitResult` _outhit)) (make `/Game/DamageSystem/Structure/S_DamageInfo` 25.0 "NewEnumerator1"))))))))

(event `/Game/Enemies/Interfaces/BPI_EnemyAI.EquipWeapon`
  ; 검을 뽑으면서 검을 생성
  (bind _notifyname (`|PlayMontage` (`self.Mesh`) "/Game/Animations/SwordAction/AM_Draw_Sword.AM_Draw_Sword")
    (:`OnCompleted`
      (`self.OnWeaponEquipped`))
    (:`OnNotifyBegin`
      (switch `name` _notifyname
        (:`HoldSword`
          (bind _returnvalue (`|SpawnActorFromClass` "/Game/Weapon/BP_Weapon_Sword.BP_Weapon_Sword_C" (`self.GetTransform`) "AlwaysSpawn" "MultiplyWithRoot" null null))
          (bind _output_get (set `self.WeaponActor` _returnvalue))
          (`self.K2_AttachToComponent` _output_get (`self.Mesh`) "hand_r_sword_socket" "SnapToTarget" "SnapToTarget" "SnapToTarget" true)
          (set `self.IsWieldingWeapon` true))))))

(event `/Game/Enemies/Interfaces/BPI_EnemyAI.UnEquipWeapon`
  ; 검을 집어 넣으면서 검을 삭제
  (bind _notifyname (`|PlayMontage` (`self.Mesh`) "/Game/Animations/SwordAction/AM_Sheath_Sword.AM_Sheath_Sword")
    (:`OnCompleted`
      (`self.OnWeaponUnEquipped`))
    (:`OnNotifyBegin`
      (switch `name` _notifyname
        (:`DropSword`
          (`self.K2_DestroyActor` (`self.WeaponActor`))
          (set `self.IsWieldingWeapon` false))))))

(fn `UserConstructionScript`
  (`parent.UserConstructionScript`))